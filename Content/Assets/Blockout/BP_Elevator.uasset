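; Blockout elevator that carries a Pivot component between two marker transforms when a Player-tagged actor enters its Box trigger.
; After a short delay, the ElevatorUp timeline drives a transform lerp from PositionA to PositionB, applied as an unswept teleport.
; When the timeline finishes, a pause leads into the ElevatorPointReached event, which reverses the timeline to send the Pivot back.
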(event `self.Box.OnComponentBeginOverlap`
  (params (OverlappedComponent :type "PrimitiveComponent Object Reference") (OtherActor :type "Actor Object Reference") (OtherComp :type "PrimitiveComponent Object Reference") (OtherBodyIndex :type Integer) (bFromSweep :type Boolean) (SweepResult :type "HitResult Structure (by ref)"))
  (if (`self.ActorHasTag` OtherActor "Player")
    (`KismetSystemLibrary.Delay` 0.5)
    (bind (_direction _elivator_hight) (`Timeline|Elevator Up` :!label _label)
      (:`Update`
        (`SceneComponent.K2_SetWorldTransform` (`self.Pivot`) (`KismetMathLibrary.TLerp` (`SceneComponent.K2_GetComponentToWorld` (`self.PositionA`)) (`SceneComponent.K2_GetComponentToWorld` (`self.PositionB`)) _elivator_hight) false true))
      (:`Finished`
        (`KismetSystemLibrary.Delay` 2.0)
        (`self.Elevator Point Reached`)))))

(event `Elevator Point Reached`
  (goto _label :!via `Reverse`))

(fn `UserConstructionScript`)