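; BP_Collectable is a pickup actor that increments the Collectable count on BP_Player when the player overlaps its Trigger.
; The overlap also spawns the pooled NS_Collectable Niagara effect and plays the CoinMove timeline, which slides the Sphere's relative location toward MoveLocation.
; The destroy and sound nodes are disconnected, so the actor persists and nothing guards against repeat pickups.
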(event `self.Trigger.OnComponentBeginOverlap`
  (params (OverlappedComponent :type "PrimitiveComponent Object Reference") (OtherActor :type "Actor Object Reference") (OtherComp :type "PrimitiveComponent Object Reference") (OtherBodyIndex :type Integer) (bFromSweep :type Boolean) (SweepResult :type "HitResult Structure (by ref)"))
  (bind _asbp_player (cast `/Game/Characer/BP_Player` OtherActor))
  (set `/Game/Characer/BP_Player.Collectable` (+ (`/Game/Characer/BP_Player.Collectable` _asbp_player) 1) _asbp_player)
  (`NiagaraFunctionLibrary.SpawnSystemAtLocation` "/Game/NiagaraSystem/NS_Collectable.NS_Collectable" (`self.K2_GetActorLocation`) (struct) (1.0 1.0 1.0) true true "AutoRelease")
  (bind (_direction _move) (`Timeline|CoinMove`)
    (:`Update`
      (`self.NewLocation` _move))))

(fn `NewLocation`
  (params (MovePercentage :type "Float (double-precision)"))
  (`SceneComponent.K2_SetRelativeLocation` (`self.Sphere`) (* MovePercentage (`self.MoveLocation`)) false false))

(fn `UserConstructionScript`)