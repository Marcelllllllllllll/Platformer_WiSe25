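; BP_TimedSpikeTrap is a spike trap that automatically extends and retracts on a repeating timer.
; On BeginPlay it scales the SpikeMovement timeline's play rate by SpikeMoveDuration, then starts the cycle.
; A FlipFlop alternates playing the timeline forward and in reverse, driving the Pivot's relative Z up to MaxExtendDistance.
; Each finish waits DelayBetweenMovement before re-triggering the event, forming an endless loop.
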(event `self.ReceiveBeginPlay`
  (`TimelineComponent.SetPlayRate` (`self.SpikeMovement`) (/ 1.0 (`self.Spike Move Duration`)))
  (`self.TriggeredSpikeChange`))

(event `TriggeredSpikeChange`
  (`/Engine/EditorBlueprintResources/StandardMacros.FlipFlop`
    (:`A`
      (bind (_direction _extendpercentage) (`Timeline|SpikeMovement` :!via `PlayFromStart` :!label _label)
        (:`Update`
          (`SceneComponent.K2_SetRelativeLocation` (`self.Pivot`) (`KismetMathLibrary.MakeVector` 0.0 0.0 (* _extendpercentage (`self.MaxExtendDistance`))) false false))
        (:`Finished`
          (`KismetSystemLibrary.Delay` (`self.DelayBetweenMovement`))
          (`self.TriggeredSpikeChange`))))
    (:`B`
      (goto _label :!via `ReverseFromEnd`))))

(fn `UserConstructionScript`)