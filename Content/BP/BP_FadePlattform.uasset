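; BP_FadePlattform is a platform that changes its opacity while a BP_Player is inside its Box trigger.
; At BeginPlay it creates a dynamic instance of MI_FadingPlattform on the Cube and disables its shadow casting.
; Player overlap plays a Timeline that drives the material's Opacity Strength parameter, and leaving reverses it for a smooth fade.
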(event `self.ReceiveBeginPlay`
  (bind _returnvalue (`PrimitiveComponent.CreateDynamicMaterialInstance` (`self.Cube`) 0 "/Game/Material/MI_FadingPlattform.MI_FadingPlattform" "None"))
  (set `self.DynamicMaterial` _returnvalue)
  (`PrimitiveComponent.SetCastShadow` (`self.Cube`) false))

(event `self.Box.OnComponentBeginOverlap`
  (params (OverlappedComponent :type "PrimitiveComponent Object Reference") (OtherActor :type "Actor Object Reference") (OtherComp :type "PrimitiveComponent Object Reference") (OtherBodyIndex :type Integer) (bFromSweep :type Boolean) (SweepResult :type "HitResult Structure (by ref)"))
  (cast `/Game/Characer/BP_Player` OtherActor)
  (set `self.IsInCollider` true)
  (bind (_direction _alpha) (`Timeline|Timeline` :!label _label)
    (:`Update`
      (`MaterialInstanceDynamic.SetScalarParameterValue` (`self.DynamicMaterial`) "Opacity Strength" _alpha))))

(event `self.Box.OnComponentEndOverlap`
  (params (OverlappedComponent :type "PrimitiveComponent Object Reference") (OtherActor :type "Actor Object Reference") (OtherComp :type "PrimitiveComponent Object Reference") (OtherBodyIndex :type Integer))
  (cast `/Game/Characer/BP_Player` OtherActor)
  (set `self.IsInCollider` false)
  (goto _label :!via `Reverse`))

(fn `UserConstructionScript`)