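; BP_DoorKeyCard is a sliding door that moves vertically with an electric garage sound; it contains no key card check itself.
; OpenDoor plays the MoveOpenDoor timeline, scaling EndLocation by its curve to set the door's relative Z.
; On Finished the sound stops and DoorClosed waits briefly, restarts it and reverses the timeline.
; Finished also follows the reverse, so DoorClosed runs again after closing.
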(event `OpenDoor`
  (bind _returnvalue (`GameplayStatics.SpawnSoundAttached` "/Game/Sound/ES_Garage__Door__Electric__Close_-_Epidemic_Sound.ES_Garage__Door__Electric__Close_-_Epidemic_Sound" (`self.Door`) "None" (0.0 0.0 0.0) (struct) "KeepRelativeOffset" false 1.0 1.0 0.0 null null false))
  (set `self.DoorSoundCop` _returnvalue)
  (bind (_direction _positiongate_z) (`Timeline|MoveOpenDoor` :!label _label)
    (:`Update`
      (`SceneComponent.K2_SetRelativeLocation` (`self.Door`) (`KismetMathLibrary.MakeVector` 0.0 0.0 (* _positiongate_z (`self.EndLocation`))) false false))
    (:`Finished`
      (`AudioComponent.Stop` (`self.DoorSoundCop`))
      (`self.DoorClosed`))))

(event `DoorClosed`
  (`KismetSystemLibrary.Delay` 2.0)
  (`AudioComponent.Play` (`self.DoorSoundCop`) 0.0)
  (goto _label :!via `Reverse`))

(fn `UserConstructionScript`)