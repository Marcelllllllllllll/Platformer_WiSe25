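; BP_JumpPlattform is a jump pad that launches the player forward and upward once it is active.
; A box overlap by BP_Player launches player character 0 along the pad's forward vector by LaunchDistance plus LaunchHight vertically, overriding existing velocity.
; The CollectableInteract event sets IsActive and swaps the Jumppad material to its "on" look.
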(event `self.Box.OnComponentBeginOverlap`
  (params (OverlappedComponent :type "PrimitiveComponent Object Reference") (OtherActor :type "Actor Object Reference") (OtherComp :type "PrimitiveComponent Object Reference") (OtherBodyIndex :type Integer) (bFromSweep :type Boolean) (SweepResult :type "HitResult Structure (by ref)"))
  (if (`self.IsActive`)
    (cast `/Game/Characer/BP_Player` OtherActor)
    (`Character.LaunchCharacter` (`GameplayStatics.GetPlayerCharacter` 0) (+ (* (`self.GetActorForwardVector`) (`self.LaunchDistance`)) (`KismetMathLibrary.MakeVector` 0.0 0.0 (`self.LaunchHight`))) true true)))

(event `/Game/BP/BPI_Plattform.CollectableInteract`
  (set `self.IsActive` true)
  (`PrimitiveComponent.SetMaterial` (`self.Jumppad`) 0 "/Game/Material/MI_PlattformOn.MI_PlattformOn"))

(fn `UserConstructionScript`)