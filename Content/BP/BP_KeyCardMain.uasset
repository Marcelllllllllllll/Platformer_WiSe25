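; BP_KeyCardMain is an interactable keycard check that opens its linked door for a player holding the required card.
; Interact looks for RequiredKeyCard in the player's CollectedKeyCardID, then either calls OpenDoor on DoorRef or prints a red missing-card message.
; The Interaction component's overlap creates and shows a BPW_Interaction widget when BP_Player enters, and removes it on any end overlap.
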(event `/Game/BP/Interface/BPI_Interactable.Interact`
  (params (PlayerRef :type "/Game/Characer/BP_Player Object Reference"))
  (if (`KismetArrayLibrary.Array_Contains` (`/Game/Characer/BP_Player.CollectedKeyCardID` PlayerRef) (`self.RequiredKeyCard`))
    (`/Game/BP/BP_DoorKeyCard.OpenDoor` (`self.DoorRef`))
    (`KismetSystemLibrary.PrintString` "KeyCardCollected")
    (else
      (`KismetSystemLibrary.PrintString` "NoKeyCardCollected" true true (struct :`R` 1.0 :`A` 1.0)))))

(event `self.Interaction.OnComponentBeginOverlap`
  (params (OverlappedComponent :type "PrimitiveComponent Object Reference") (OtherActor :type "Actor Object Reference") (OtherComp :type "PrimitiveComponent Object Reference") (OtherBodyIndex :type Integer) (bFromSweep :type Boolean) (SweepResult :type "HitResult Structure (by ref)"))
  (cast `/Game/Characer/BP_Player` OtherActor)
  (bind _returnvalue (`|CreateWidget` "/Game/UI/Widgeds/BPW_Interaction.BPW_Interaction_C"))
  (bind _output_get (set `self.InteractionWidget` _returnvalue))
  (`UserWidget.AddToViewport` _output_get 0))

(event `self.Interaction.OnComponentEndOverlap`
  (params (OverlappedComponent :type "PrimitiveComponent Object Reference") (OtherActor :type "Actor Object Reference") (OtherComp :type "PrimitiveComponent Object Reference") (OtherBodyIndex :type Integer))
  (`Widget.RemoveFromParent` (`self.InteractionWidget`)))

(fn `GetInteractionWidgetRef`
  (returns (Ref :type "WidgetComponent Object Reference"))
  (return null))

(fn `UserConstructionScript`)