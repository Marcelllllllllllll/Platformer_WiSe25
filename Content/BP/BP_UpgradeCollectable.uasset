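; BP_UpgradeCollectable is a pickup that grants the player a stamina, dash, jump or health upgrade, chosen by CollectableType.
; The construction script sets mesh and material from that type.
; Box overlap with BP_Player applies the upgrade and destroys the actor; only stamina plays an effect and sound.
; Stamina and dash upgrades are also written to BP_GameInstance, while jump and health change only the player.
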(event `self.Box.OnComponentBeginOverlap`
  (params (OverlappedComponent :type "PrimitiveComponent Object Reference") (OtherActor :type "Actor Object Reference") (OtherComp :type "PrimitiveComponent Object Reference") (OtherBodyIndex :type Integer) (bFromSweep :type Boolean) (SweepResult :type "HitResult Structure (by ref)"))
  (bind _asbp_player (cast `/Game/Characer/BP_Player` OtherActor))
  (bind _asbp_game_instance (cast `/Game/BP/BP_GameInstance` (`GameplayStatics.GetGameInstance`)))
  (switch `/Game/BP/ECollectableType` (`self.CollectableType`)
    (:`NewEnumerator0`
      (bind _returnvalue (+ (`/Game/Characer/BP_Player.MaxStamina` _asbp_player) 25.0))
      (set `/Game/BP/BP_GameInstance.PlayerMaxStamina` _returnvalue _asbp_game_instance)
      (set `/Game/Characer/BP_Player.MaxStamina` _returnvalue _asbp_player)
      (`/Game/UI/Widgeds/WB_Stamina.Angle` (`/Game/Characer/BP_Player.StaminaWidged` _asbp_player))
      (`NiagaraFunctionLibrary.SpawnSystemAtLocation` "/Game/NiagaraSystem/NS_Collectable.NS_Collectable" (`self.K2_GetActorLocation`) (struct) (1.0 1.0 1.0) true true "AutoRelease")
      (`self.K2_DestroyActor`)
      (`GameplayStatics.PlaySound2D` "/Engine/VREditor/Sounds/UI/Object_Snaps_To_Grid.Object_Snaps_To_Grid" 1.0 1.0 0.0 null null))
    (:`NewEnumerator1`
      (set `/Game/BP/BP_GameInstance.DashUnlocked` true _asbp_game_instance)
      (set `/Game/Characer/BP_Player.CanDash` true _asbp_player)
      (`self.K2_DestroyActor`))
    (:`NewEnumerator2`
      (bind _result (`/Engine/EditorBlueprintResources/StandardMacros.IncrementInt` (`Character.JumpMaxCount` _asbp_player))
        (:`  `
          (set `Character.JumpMaxCount` _result _asbp_player)
          (`self.K2_DestroyActor`))))
    (:`NewEnumerator3`
      (set `/Game/Characer/BP_Player.Health` (+ (`/Game/Characer/BP_Player.Health` _asbp_player) 10.0) _asbp_player)
      (`self.K2_DestroyActor`))))

(fn `UserConstructionScript`
  (bind _mesh (`self.Mesh`))
  (bind _collectabletype (`self.CollectableType`))
  (`PrimitiveComponent.SetMaterial` _mesh 0 (select `/Game/BP/ECollectableType` _collectabletype :`NewEnumerator0` "/Game/Material/MI_CollectableStamina.MI_CollectableStamina" :`NewEnumerator1` "/Game/Material/MI_CollectableStamina.MI_CollectableStamina" :`NewEnumerator2` "/Game/Material/MI_CollectableStamina.MI_CollectableStamina" :`NewEnumerator3` "/Game/Material/MI_CollectableHealth.MI_CollectableHealth" :!type "MaterialInterface Object Reference"))
  (`StaticMeshComponent.SetStaticMesh` _mesh (select `/Game/BP/ECollectableType` _collectabletype :`NewEnumerator0` "/Game/Assets/Collectables/CollectableStamina.CollectableStamina" :`NewEnumerator1` "/Game/Assets/Collectables/CollectableDash.CollectableDash" :`NewEnumerator2` "/Game/Assets/Collectables/CollectableDoubleJump.CollectableDoubleJump" :`NewEnumerator3` "/Game/Assets/Collectables/CollectableHealth.CollectableHealth" :!type "StaticMesh Object Reference")))