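; Breakable platform that falls away once the player enters its trigger box.
; The first Box overlap by a BP_Player stores that player and calls CollapsePlatform, with a DoOnce preventing repeat triggers.
; CollapsePlatform turns on physics simulation for the Cube, then disables its collision after a short delay.
; An input-disable step for the player is present but unconnected, so it never runs.
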(event `CollapsePlatform`
  (`PrimitiveComponent.SetSimulatePhysics` (`self.Cube`) true)
  (`KismetSystemLibrary.Delay` 2.0)
  (`PrimitiveComponent.SetCollisionEnabled` (`self.Cube`) "NoCollision"))

(event `self.Box.OnComponentBeginOverlap`
  (params (OverlappedComponent :type "PrimitiveComponent Object Reference") (OtherActor :type "Actor Object Reference") (OtherComp :type "PrimitiveComponent Object Reference") (OtherBodyIndex :type Integer) (bFromSweep :type Boolean) (SweepResult :type "HitResult Structure (by ref)"))
  (bind _asbp_player (cast `/Game/Characer/BP_Player` OtherActor))
  (`/Engine/EditorBlueprintResources/StandardMacros.DoOnce` false
    (:`Completed`
      (set `self.PlayerRef` _asbp_player)
      (`self.CollapsePlatform`))))

(fn `UserConstructionScript`)