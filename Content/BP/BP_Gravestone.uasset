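; Gravestone actor that randomizes its placement and shape so copies look varied.
; BeginPlay adds a random height offset to the mesh, sets a random world rotation on the scene component and applies random per-axis scale.
; Separate functions offer relative-space XYZ offset, rotation, scale and a random mesh pick, bundled in ApplyAllVariations.
; Nothing in this graph calls that bundle, and the construction script is empty.
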(event `self.ReceiveBeginPlay`
  (bind _mesh (`self.Mesh`))
  (bind _maxrotationoffset (`self.MaxRotationOffset`))
  (bind _maxrotationoffset_2 (`self.MaxRotationOffset`))
  (bind _maxhightoffest (`self.MaxHightOffest`))
  (bind _returnvalue (`KismetMathLibrary.RandomFloatInRange` (`self.MinRandomScaleValue`) (`self.MaxRandomScaleValue`)))
  ; Zufälliger Offest (Z-Achse)
  (`SceneComponent.K2_AddWorldOffset` _mesh (`KismetMathLibrary.MakeVector` 0.0 0.0 (`KismetMathLibrary.RandomFloatInRange` (* _maxhightoffest -1.0) _maxhightoffest)) false false)
  ; Zufällige Rotation (XYZ-Achse)
  (`SceneComponent.K2_SetWorldRotation` (`self.Scene`) (`KismetMathLibrary.MakeRotator` (`KismetMathLibrary.RandomFloatInRange` (* _maxrotationoffset_2 -1.0) _maxrotationoffset_2) (`KismetMathLibrary.RandomFloatInRange` (* _maxrotationoffset -1.0) _maxrotationoffset) (`KismetMathLibrary.RandomFloatInRange` 0.0 (`self.RandomRotationValue`))) false false)
  ; Zufällige Größe (20% größer oder kleiner)
  (`SceneComponent.SetRelativeScale3D` _mesh (`KismetMathLibrary.MakeVector` _returnvalue _returnvalue _returnvalue)))

(fn `ApplyAllVariations`
  (`self.Random Z-Offset`)
  (`self.RandomYawRollAndPitch`)
  (`self.RandomScale`)
  (`self.SetRandomMesh`))

(fn `Random Z-Offset`
  (bind _maxhightoffest (`self.MaxHightOffest`))
  (bind _maxxyoffset (`self.MaxXYOffset`))
  (bind _maxxyoffset_2 (`self.MaxXYOffset`))
  (`SceneComponent.K2_SetRelativeLocation` (`self.Mesh`) (`KismetMathLibrary.MakeVector` (`KismetMathLibrary.RandomFloatInRange` (* _maxxyoffset_2 -1.0) _maxxyoffset_2) (`KismetMathLibrary.RandomFloatInRange` (* _maxxyoffset -1.0) _maxxyoffset) (`KismetMathLibrary.RandomFloatInRange` (* _maxhightoffest -1.0) _maxhightoffest)) false false)
  (return))

(fn `RandomScale`
  (bind _returnvalue (`KismetMathLibrary.RandomFloatInRange` (`self.MinRandomScaleValue`) (`self.MaxRandomScaleValue`)))
  (`SceneComponent.SetRelativeScale3D` (`self.Mesh`) (`KismetMathLibrary.MakeVector` _returnvalue _returnvalue _returnvalue)))

(fn `RandomYawRollAndPitch`
  (bind _maxrotationoffset (`self.MaxRotationOffset`))
  (bind _maxrotationoffset_2 (`self.MaxRotationOffset`))
  (`SceneComponent.K2_SetRelativeRotation` (`self.Scene`) (`KismetMathLibrary.MakeRotator` (`KismetMathLibrary.RandomFloatInRange` (* _maxrotationoffset_2 -1.0) _maxrotationoffset_2) (`KismetMathLibrary.RandomFloatInRange` (* _maxrotationoffset -1.0) _maxrotationoffset) (`KismetMathLibrary.RandomFloatInRange` 0.0 (`self.RandomRotationValue`))) false false))

(fn `SetRandomMesh`
  (`StaticMeshComponent.SetStaticMesh` (`self.Mesh`) (`KismetArrayLibrary.Array_Random` (`self.New Mesh`))))

(fn `UserConstructionScript`)