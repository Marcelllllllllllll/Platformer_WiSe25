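; BP_BrainLevelCore is a brain level core actor that opens a BPW_BrainCoreScreen widget when the player touches it.
; From BeginPlay, the CoreRotation timeline spins the cube by combining each update's yaw value with its current relative rotation.
; When BP_Player overlaps the box, it adds the widget to the viewport, switches to UI-only input with a visible cursor and pauses the game.
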(event `self.ReceiveBeginPlay`
  (bind _cube (`self.Cube`))
  (bind _cube_2 (`self.Cube`))
  (`SceneComponent.K2_SetRelativeRotation` _cube_2 (`SceneComponent.RelativeRotation` _cube_2) false false)
  (bind (_direction _rotation) (`Timeline|Core rotation`)
    (:`Update`
      (set `self.StartRotation` (`SceneComponent.RelativeRotation` _cube))
      (`SceneComponent.K2_SetRelativeRotation` _cube (`KismetMathLibrary.ComposeRotators` (`self.StartRotation`) (`KismetMathLibrary.MakeRotator` 0.0 0.0 _rotation)) false false))))

(event `self.Box.OnComponentBeginOverlap`
  (params (OverlappedComponent :type "PrimitiveComponent Object Reference") (OtherActor :type "Actor Object Reference") (OtherComp :type "PrimitiveComponent Object Reference") (OtherBodyIndex :type Integer) (bFromSweep :type Boolean) (SweepResult :type "HitResult Structure (by ref)"))
  (bind _returnvalue (`GameplayStatics.GetPlayerController` 0))
  (cast `/Game/Characer/BP_Player` OtherActor)
  (bind _returnvalue_2 (`|CreateWidget` "/Game/UI/Widgeds/BPW_BrainCoreScreen.BPW_BrainCoreScreen_C" _returnvalue))
  (bind _output_get (set `self.BrainCoreWidget` _returnvalue_2))
  (`UserWidget.AddToViewport` _output_get 0)
  (`WidgetBlueprintLibrary.SetInputMode_UIOnlyEx` _returnvalue _output_get)
  (set `PlayerController.bShowMouseCursor` true _returnvalue)
  (`GameplayStatics.SetGamePaused` true))

(fn `UserConstructionScript`)