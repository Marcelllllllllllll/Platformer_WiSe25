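; BP_MyFirstBlueprint is a practice actor with a mesh that rises continuously and a point light that changes at random.
; On BeginPlay, ModifyMesh prints a greeting and calls NewFunction to nudge, rotate, rescale and swap the mesh.
; Tick moves the mesh upward scaled by delta time, prints a debug string, and uses a Delay to randomize light color and intensity about once per second.
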(event `ModifyMesh`
  (`KismetSystemLibrary.PrintString` "Hello World!" true true (struct :`G` 0.66 :`B` 1.0 :`A` 1.0) 6.0)
  (`self.NewFunction`))

(event `self.ReceiveBeginPlay`
  (`self.ModifyMesh`))

(event `self.ReceiveActorBeginOverlap`
  (params (OtherActor :type "Actor Object Reference"))
  ; Trigger and Collision
)

(event `self.ReceiveTick`
  (params (DeltaSeconds :type "Float (single-precision)"))
  (bind _pointlight (`self.PointLight`))
  (`SceneComponent.K2_AddWorldOffset` (`self.Mesh`) (* (0.0 0.0 50.0) DeltaSeconds) false false)
  (`KismetSystemLibrary.PrintString` "IsGrounded" true true (struct :`G` 0.66 :`B` 1.0 :`A` 1.0) 0.0)
  (`KismetSystemLibrary.Delay` 1.0)
  (`LightComponent.SetLightColor` _pointlight (make `LinearColor` (`KismetMathLibrary.RandomFloatInRange` 0.0 1.0) (`KismetMathLibrary.RandomFloatInRange` 0.0 360.0) (`KismetMathLibrary.RandomFloatInRange` 0.0 1.0) 1.0) true)
  (`LightComponent.SetIntensity` _pointlight (`KismetMathLibrary.RandomFloatInRange` 50.0 100.0)))

(event `self.ReceiveHit`
  (params (MyComp :type "PrimitiveComponent Object Reference") (Other :type "Actor Object Reference") (OtherComp :type "PrimitiveComponent Object Reference") (bSelfMoved :type Boolean) (HitLocation :type "Vector Structure") (HitNormal :type "Vector Structure") (NormalImpulse :type "Vector Structure") (Hit :type "HitResult Structure (by ref)"))
  ; Trigger and Collision
)

(fn `NewFunction`
  (bind _mesh (`self.Mesh`))
  (`SceneComponent.K2_AddWorldOffset` _mesh (0.0 0.0 10.0) false false)
  (`SceneComponent.K2_AddWorldRotation` _mesh (struct :`Yaw` 20.0) false false)
  (`SceneComponent.SetWorldScale3D` _mesh (0.5 0.5 1.0))
  (`StaticMeshComponent.SetStaticMesh` _mesh "/Engine/EditorMeshes/EditorHelp.EditorHelp"))

(fn `UserConstructionScript`)