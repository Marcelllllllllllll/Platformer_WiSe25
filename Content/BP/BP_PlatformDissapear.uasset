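; Platform Blueprint, named as a disappearing platform, that lights up its material when something overlaps its Box trigger.
; On BeginPlay it creates a dynamic material instance on the mesh and zeroes its base color and emission strength.
; Any overlap raises both parameters and plays Opacity, though the graph shows no update logic, collision change or reset for it.
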(event `self.ReceiveBeginPlay`
  (bind _returnvalue (`PrimitiveComponent.CreateDynamicMaterialInstance` (`self.Mesh`) 0 "/Game/Material/M_DissapearPlattform.M_DissapearPlattform" "None"))
  (bind _output_get (set `self.Dynamical Material` _returnvalue))
  (`MaterialInstanceDynamic.SetScalarParameterValue` _output_get "BaseColorStrenght" 0.0)
  (`MaterialInstanceDynamic.SetScalarParameterValue` _output_get "EmissionStrenght" 0.0))

(event `self.Box.OnComponentBeginOverlap`
  (params (OverlappedComponent :type "PrimitiveComponent Object Reference") (OtherActor :type "Actor Object Reference") (OtherComp :type "PrimitiveComponent Object Reference") (OtherBodyIndex :type Integer) (bFromSweep :type Boolean) (SweepResult :type "HitResult Structure (by ref)"))
  (bind _dynamical_material (`self.Dynamical Material`))
  (`MaterialInstanceDynamic.SetScalarParameterValue` _dynamical_material "BaseColorStrenght" 5.0)
  (`MaterialInstanceDynamic.SetScalarParameterValue` _dynamical_material "EmissionStrenght" 1.0)
  (`|ExecutionSequence`
    (:`then_0`
      (`Timeline|Opacity`))))

(fn `UserConstructionScript`)