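; BP_DamageZone is a box trigger zone meant to deal periodic damage to BP_Player while it stays inside.
; Begin overlap stores the player and starts a looping timer at the damage interval, and end overlap clears that timer.
; DealZoneDamage applies the damage amount to the stored player if valid.
; DisableZone is empty, with timer-clear and destroy nodes left unconnected.
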(event `DisableZone`)

(event `DealZoneDamage`
  (bind _playerref (`self.PlayerRef`))
  (`/Engine/EditorBlueprintResources/StandardMacros.IsValid` _playerref
    (:`Is Valid`
      (`GameplayStatics.ApplyDamage` _playerref (`self.DamageAmount`)))))

(event `self.Box.OnComponentBeginOverlap`
  (params (OverlappedComponent :type "PrimitiveComponent Object Reference") (OtherActor :type "Actor Object Reference") (OtherComp :type "PrimitiveComponent Object Reference") (OtherBodyIndex :type Integer) (bFromSweep :type Boolean) (SweepResult :type "HitResult Structure (by ref)"))
  (bind _asbp_player (cast `/Game/Characer/BP_Player` OtherActor))
  (set `self.PlayerRef` _asbp_player)
  (bind _returnvalue (`KismetSystemLibrary.K2_SetTimerDelegate` (`|CreateDelegate` :!event `DealZoneDamage`) (`self.DamageInterval`) true))
  (set `self.DamageTimerHandle` _returnvalue))

(event `self.Box.OnComponentEndOverlap`
  (params (OverlappedComponent :type "PrimitiveComponent Object Reference") (OtherActor :type "Actor Object Reference") (OtherComp :type "PrimitiveComponent Object Reference") (OtherBodyIndex :type Integer))
  (cast `/Game/Characer/BP_Player` OtherActor)
  (`KismetSystemLibrary.K2_ClearAndInvalidateTimerHandle` (`self.DamageTimerHandle`)))

(fn `UserConstructionScript`)